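; Base actor for a moving line of coloured blocks that projectiles recolour to score points.
; Tick moves the line along its forward vector until dead, with materials looked up from each block's colour.
; BlockHit copies the projectile's colour to the struck block, then checks whether all blocks match.
; A match adds score, launches the blocks with physics, calls LineDeath and destroys the actor after a delay; Despawnblocks removes it immediately.
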(event Custom|Destroy%20Blocks
  ;[1 1 1] destroy
  (Utilities|FlowControl|Delay 1e+01)
  (Actor|DestroyActor))

(event Custom|Despawn%20blocks
  (Default|CallLineDeath)
  (Actor|DestroyActor))

(event EventBeginPlay
  (for (_array_element _array_index) (Variables|Default|GetBlocks)
    (Rendering|Material|SetMaterial _array_element 0 (Utilities|Array|Get(acopy) (Variables|Default|GetM_Colours) (Math|Conversions|ToInteger(Byte) (Utilities|Array|Get(acopy) (Variables|Default|GetBlockColours) _array_index))))
    (Collision|SetCollisionProfileName _array_element "Blocks" :!class /Script/Engine.PrimitiveComponent)))

(event Collision|EventActorBeginOverlap
  (params (OtherActor :type Actor%20Object%20Reference)))

(event EventTick
  (params (DeltaSeconds :type Float%20%28single-precision%29))
  ;[1 1 1] Movement
  (if (not (Variables|Default|GetDead?))
    (Transformation|AddActorWorldOffset (* (Transformation|GetActorForwardVector) (* DeltaSeconds (Variables|Default|GetSpeed))))))

(fn ConstructionScript)

(fn SameColour?
  (bind _array_index (Utilities|Array|ForEachLoopwithBreak (Variables|Default|GetBlocks) :!label _label)
    (:LoopBody
      (if (== (Utilities|Array|Get(acopy) (Variables|Default|GetBlockColours) _array_index) (Utilities|Array|Get(acopy) (Variables|Default|GetBlockColours)))
        (LocalVariables|SetFullMatch? true)
        (else
          (LocalVariables|SetFullMatch? false)
          (goto _label Break))))
    (:Completed
      (return (LocalVariables|GetFullMatch?)))))

(fn BlockHit
  (params (Hit%20Component :type Static%20Mesh%20Component%20Object%20Reference%20%28by%20ref%29) (Other%20actor :type Object%20Object%20Reference))
  (bind _returnvalue (Transformation|GetActorLocation))
  ;[1 1 1] Handle pprojectile Hit
  (Development|PrintString "Hit")
  (bind _asprojectile (Utilities|Casting|CastToProjectile Other%20actor))
  (Utilities|Array|SetArrayElem (Variables|Default|GetBlockColours) (Utilities|Array|FindItem (Variables|Default|GetBlocks) Hit%20Component) (Variables|/Game/BP/Projectile.Projectile_C|GetColour _asprojectile))
  (Rendering|Material|SetMaterial Hit%20Component 0 (Utilities|Array|Get(acopy) (Variables|Default|GetM_Colours) (Math|Conversions|ToInteger(Byte) (Variables|/Game/BP/Projectile.Projectile_C|GetColour _asprojectile))))
  (Actor|DestroyActor _asprojectile)
  ;[1 1 1] Same colours?
  (bind _result (CallFunction|SameColour?))
  (if _result
    (bind _scoreboard (Variables|Default|GetScoreboard)
      (:then
        (Default|ChangeScore _scoreboard (Variables|Default|GetScoreWorth)))
      (:else
        (Development|PrintString "no scoreboard")))
    ;[1 1 1] Flip out blocks
    (for _array_element (Variables|Default|GetBlocks)
      (Collision|SetCollisionProfileName _array_element "DeadBlock" :!class /Script/Engine.PrimitiveComponent)
      (Physics|SetSimulatePhysics _array_element true)
      (Physics|AddImpulseatLocation _array_element "0.0,0.0,300000.000000" (Math|Vector|MakeVector (.x _returnvalue) (+ (.y _returnvalue) (Math|Random|RandomFloatinRange -2e+02 2e+02)) (.z _returnvalue)) "None"))
    ;[1 1 1] Finish up
    (Audio|PlaySound2D "/Game/Blockexsplosion.Blockexsplosion" 1.0 1.0 0.0 0 0)
    (Variables|Default|SetDead? true)
    (Default|CallLineDeath)
    (CallFunction|DestroyBlocks)))