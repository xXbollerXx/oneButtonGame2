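; BP_3BlockLine is a child Blueprint for a line of three blocks that respond to being hit.
; On BeginPlay it fills a Blocks array with its Block2, Block3 and Block4 components, then runs the parent's BeginPlay.
; Each block's component hit event forwards that block and the other actor to a shared BlockHit call, whose logic is not defined here.
; The construction script does nothing, as its array setup and parent call are disconnected.
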(event OnComponentHit(Block3)
  (params (HitComponent :type Primitive%20Component%20Object%20Reference) (OtherActor :type Actor%20Object%20Reference) (OtherComp :type Primitive%20Component%20Object%20Reference) (NormalImpulse :type Vector :default "0, 0, 0") (Hit :type Hit%20Result%20Structure%20%28by%20ref%29))
  (CallFunction|BlockHit (Variables|Default|GetBlock3) OtherActor))

(event OnComponentHit(Block4)
  (params (HitComponent :type Primitive%20Component%20Object%20Reference) (OtherActor :type Actor%20Object%20Reference) (OtherComp :type Primitive%20Component%20Object%20Reference) (NormalImpulse :type Vector :default "0, 0, 0") (Hit :type Hit%20Result%20Structure%20%28by%20ref%29))
  (CallFunction|BlockHit (Variables|Default|GetBlock4) OtherActor))

(event OnComponentHit(Block2)
  (params (HitComponent :type Primitive%20Component%20Object%20Reference) (OtherActor :type Actor%20Object%20Reference) (OtherComp :type Primitive%20Component%20Object%20Reference) (NormalImpulse :type Vector :default "0, 0, 0") (Hit :type Hit%20Result%20Structure%20%28by%20ref%29))
  (CallFunction|BlockHit (Variables|Default|GetBlock2) OtherActor))

(event EventBeginPlay
  (Variables|Default|SetBlocks (Utilities|Array|MakeArray (Variables|Default|GetBlock2) (Variables|Default|GetBlock3) (Variables|Default|GetBlock4)))
  (|CallParentFunction))

(event Collision|EventActorBeginOverlap
  (params (OtherActor :type Actor%20Object%20Reference)))

(fn ConstructionScript)